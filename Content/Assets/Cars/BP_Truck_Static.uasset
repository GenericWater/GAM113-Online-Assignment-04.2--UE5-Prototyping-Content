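; Drivable truck that moves by physics force on its TruckBody and carries a player-rotated spring-arm camera.
; BeginPlay zeroes the body's linear and angular velocity.
; The MoveForward axis and Tick share one path that pushes the body along its forward vector, scaled by input and DriveForce, and debug-prints the axis value.
; TurnCamera yaws the spring arm; no steering logic is present.
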(event EventBeginPlay
  (bind _truckbody (Variables|Default|GetTruckBody))
  (Physics|SetPhysicsLinearVelocity _truckbody "0, 0, 0" false "None")
  (Class|PrimitiveComponent|SetPhysicsAngularVelocityinDegrees _truckbody "0, 0, 0" false "None"))

(event Collision|EventActorBeginOverlap
  (params (OtherActor :type Actor%20Object%20Reference)))

(event EventTick
  (params (DeltaSeconds :type Float%20%28single-precision%29))
  (Physics|AddForce (Variables|Default|GetTruckBody) (* (stale Input|AxisEvents|InputAxisMoveForward AxisValue) (Math|Vector|GetForwardVector (Variables|Default|GetTruckBody)) (Variables|Default|GetDriveForce)) "None" false)
  (Development|PrintString (Utilities|String|ToString(Float) (stale Input|AxisEvents|InputAxisMoveForward AxisValue))))

(event Input|AxisEvents|InputAxisTurnCamera
  (params (AxisValue :type Float%20%28single-precision%29))
  ;[0.15 0.15 0.15 0.5] Camera Movement
  (Transformation|AddRelativeRotation (Variables|Default|GetSpringArm) (Math|Rotator|MakeRotator 0.0 0.0 (* AxisValue 2.0)) false false))

(event Input|AxisEvents|InputAxisMoveForward
  (params (AxisValue :type Float%20%28single-precision%29))
  (Physics|AddForce (Variables|Default|GetTruckBody) (* AxisValue (Math|Vector|GetForwardVector (Variables|Default|GetTruckBody)) (Variables|Default|GetDriveForce)) "None" false)
  (Development|PrintString (Utilities|String|ToString(Float) AxisValue)))

(fn ConstructionScript)